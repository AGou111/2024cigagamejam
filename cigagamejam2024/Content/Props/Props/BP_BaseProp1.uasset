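; BP_BaseProp1 is a base prop actor that acts as a one-shot overlap trigger, sending an event to whatever touches it.
; On BeginPlay it binds to its Capsule's begin-overlap event.
; An overlapping actor that implements BPI_Msg receives PropEventMessage with the prop's EventName, then the prop destroys itself.
; A Live flag is cleared before sending so the message fires only once.
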(event Custom|CustomEvent
  (params (OverlappedComponent :type Primitive%20Component%20Object%20Reference) (OtherActor :type Actor%20Object%20Reference) (OtherComp :type Primitive%20Component%20Object%20Reference) (OtherBodyIndex :type Integer) (bFromSweep :type Boolean) (SweepResult :type Hit%20Result%20Structure%20%28by%20ref%29))
  (if (Utilities|DoesObjectImplementInterface OtherActor "/Game/Props/BPI_Msg.BPI_Msg_C")
    (if (Variables|Default|GetLive)
      (Variables|Default|SetLive false)
      (Class|BPIMsg|PropEvent(Message) OtherActor (Variables|配置项|GetEventName))
      (Actor|DestroyActor))))

(event EventBeginPlay
  (Collision|BindEventtoOnComponentBeginOverlap (Variables|Default|GetCapsule) (delegate Custom|CustomEvent)))

(fn ConstructionScript)