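; BP_BaseProp is a base pickup prop that fires once when an actor implementing BPI_Msg overlaps it.
; On BeginPlay, ShowOrHideActor sets it live, shows its Niagara effect and binds the capsule's overlap event.
; A valid overlap sends EventName to that actor through PropEventMessage, plays a 2D sound, then hides the effect and unbinds the overlap.
; The prop is hidden rather than destroyed.
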(event Custom|吃道具
  (params (OverlappedComponent :type Primitive%20Component%20Object%20Reference) (OtherActor :type Actor%20Object%20Reference) (OtherComp :type Primitive%20Component%20Object%20Reference) (OtherBodyIndex :type Integer) (bFromSweep :type Boolean) (SweepResult :type Hit%20Result%20Structure%20%28by%20ref%29))
  (if (Utilities|DoesObjectImplementInterface OtherActor "/Game/Props/BPI_Msg.BPI_Msg_C")
    (if (Variables|Default|GetLive)
      (Variables|Default|SetLive false)
      (Class|BPIMsg|PropEvent(Message) OtherActor (Variables|配置项|GetEventName))
      (Audio|PlaySound2D (Variables|配置项|GetSound) 1.0 1.0 0.0 0 0)
      (CallFunction|ShoworHideActor false))))

(event EventBeginPlay
  (CallFunction|ShoworHideActor true))

(fn ConstructionScript)

(fn ShoworHideActor
  (params (Show :type Boolean))
  (if Show
    (Variables|Default|SetLive true)
    (Rendering|SetVisibility (Variables|Default|GetNiagara) true false)
    (Collision|BindEventtoOnComponentBeginOverlap (Variables|Default|GetCapsule) (EventDispatchers|CreateEvent :!event Custom|吃道具))
    (else
      (Variables|Default|SetLive false)
      (Rendering|SetVisibility (Variables|Default|GetNiagara) false false)
      (EventDispatchers|UnbindallEventsfromOnComponentBeginOverlap (Variables|Default|GetCapsule)))))