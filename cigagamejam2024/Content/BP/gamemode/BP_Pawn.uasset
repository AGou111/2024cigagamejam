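; Player ball pawn for an endless bouncing game along Y, launched from a swinging aim arrow and lost on leaving a boundary box.
; Tick clamps speed, moves the root and trailing back paddle, and spawns random map chunks by distance tier, removing old ones.
; Hits add speed, camera shake, effects and timeline-driven mesh squash.
; Prop events grant coins, speed boosts, longer paddles or a centering shield dash, with stats sent to the gameplay UI.
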(event Custom|LaunchBall
  (Effects|SpawnEmitterAttached "/Game/VFX/Gas/Particles/TuoWei.TuoWei" (Variables|Collision|GetCapsuleComponent) "None")
  (if (not (Variables|Default|GetLaunched))
    (Variables|Default|SetLaunched true)
    (Physics|SetPhysicsLinearVelocity (Variables|Collision|GetCapsuleComponent) (* (* (Variables|Default|Getforce) -1.0) (Math|Vector|Normalize (Math|Rotator|GetRotationXVector (Transformation|GetWorldRotation (Variables|Default|Getjiantou))))) false "None")
    (Components|DestroyComponent (Variables|Default|Getjiantou))
    (|CollapseGraph) ; enters at StopTimeline
  ))

(event Custom|失败界面
  (params (OverlappedComponent :type Primitive%20Component%20Object%20Reference) (OtherActor :type Actor%20Object%20Reference) (OtherComp :type Primitive%20Component%20Object%20Reference) (OtherBodyIndex :type Integer))
  (if (Class|GameplayStatics|ObjectIsA OtherActor "BP_Pawn_C")
    (CallFunction|Defeated)
    (Utilities|FlowControl|Delay 3.0)
    (Physics|SetPhysicsLinearVelocity (Variables|Collision|GetCapsuleComponent) "0, 0, 0" false "None")))

(event Custom|DoPerSec
  (bind _as_bp_pcontroller (CallFunction|GetPcontroller))
  (bind _ui_gameplay (Variables|/Game/BP/gamemode/BP_PController.BP_PController_C|GetUI_GamePlay _as_bp_pcontroller))
  (Default|UIMsg _ui_gameplay "speed" (.y (Transformation|GetComponentVelocity (Variables|Collision|GetCapsuleComponent))))
  (Default|UIMsg _ui_gameplay "distance" (Variables|Default|GetBallLocationY)))

(event EventBeginPlay
  (Utilities|FlowControl|Sequence
    (:then_0
      (|CollapseGraph))
    (:then_1
      (Transformation|DetachFromComponent (Variables|Default|GetRoot) "KeepWorld" "KeepWorld" "KeepWorld" true)
      (Collision|BindEventtoOnComponentEndOverlap (Variables|Default|GetBox) (delegate Custom|失败界面)))
    (:then_2
      (Utilities|Time|SetTimerbyEvent (delegate Custom|DoPerSec) 0.5 true true))))

(event EventPropEvent
  (params (EventName :type Name :default "None"))
  (switch name EventName
    (:Coin
      (CallFunction|AddCoins 1))
    (:Gem
      (CallFunction|AddCoins 1))
    (:Speed
      (|球提速))
    (:Length
      (Default|挡板变长 (CallFunction|GetPcontroller)))
    (:Shield
      (|护盾冲刺))))

(event EventTick
  (params (DeltaSeconds :type Float%20%28single-precision%29))
  (Utilities|FlowControl|Sequence
    (:then_0
      (|如果速度过大则重设速度))
    (:then_1
      (|关卡生成逻辑))
    (:then_2
      (|移动Root))
    (:then_3
      (|挡板位置逻辑))
    (:then_4
      (|翻滚转向))))

(event Collision|EventHit
  (params (MyComp :type Primitive%20Component%20Object%20Reference) (Other :type Actor%20Object%20Reference) (OtherComp :type Primitive%20Component%20Object%20Reference) (bSelfMoved :type Boolean) (HitLocation :type Vector :default "0, 0, 0") (HitNormal :type Vector :default "0, 0, 0") (NormalImpulse :type Vector :default "0, 0, 0") (Hit :type Hit%20Result%20Structure%20%28by%20ref%29))
  (Utilities|FlowControl|Sequence
    (:then_0
      (|碰撞后加速))
    (:then_1
      (|相机抖动))
    (:then_2
      (|播特效和猫头变形 HitLocation))))

(event Input|KeyboardEvents|DebugKeyM
  (params (Key :type Key%20Structure) (ActionValue :type Input%20Action%20Value%20Structure))
  (:Pressed
    (|护盾冲刺)))

(fn ConstructionScript)

(fn GetPcontroller
  (bind _as_bp_pcontroller (Variables|Default|GetAs%20BP%20PController)
    (:then
      (return _as_bp_pcontroller))
    (:else
      (bind _asbp_pcontroller (Utilities|Casting|CastToBP_PController (Game|GetPlayerController 0))
        (:then
          (bind _output_get (Variables|Default|SetAs%20BP%20PController _asbp_pcontroller))
          (return _output_get))
        (:CastFailed
          (return 0))))))

(fn Defeated
  (bind _returnvalue (UserInterface|CreateWidget "/Game/BP/UI/P_Defeated.P_Defeated_C" (Game|GetPlayerController 0)))
  (UserInterface|Viewport|AddtoViewport _returnvalue 0))

(fn AddCoins
  (params (CoinCount :type Integer))
  (bind _output_get (Variables|属性|SetCurCoins (+ CoinCount (Variables|属性|GetCurCoins))))
  (Default|UIMsg (Variables|/Game/BP/gamemode/BP_PController.BP_PController_C|GetUI_GamePlay (CallFunction|GetPcontroller)) "coin" (Math|Conversions|ToFloat(Integer) _output_get))
  (return _output_get))

(event Custom|CustomEvent_0
  (bind _capsulecomponent (Variables|Collision|GetCapsuleComponent))
  (Transformation|AddRelativeLocation _capsulecomponent (Math|Vector|MakeVector (/ (.x (Transformation|GetWorldLocation _capsulecomponent)) -25.0) 0.0 0.0) false false)
  (if (< (Math|Float|Absolute(Float) (.x (Transformation|GetWorldLocation (Variables|Collision|GetCapsuleComponent)))) 0.5)
    (Utilities|Time|ClearandInvalidateTimerbyHandle (Variables|护盾冲刺|Get护盾用临时timer))))

(event Custom|CustomEvent_1
  (params (OverlappedComponent :type Primitive%20Component%20Object%20Reference) (OtherActor :type Actor%20Object%20Reference) (OtherComp :type Primitive%20Component%20Object%20Reference) (OtherBodyIndex :type Integer) (bFromSweep :type Boolean) (SweepResult :type Hit%20Result%20Structure%20%28by%20ref%29))
  (if (Class|GameplayStatics|ObjectIsA OtherActor "/Game/Props/Props/BP_BaseProp.BP_BaseProp_C")
    (Transformation|SetActorLocation (Transformation|GetWorldLocation (Variables|Collision|GetCapsuleComponent)) false false)))