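; Player controller that spawns a paddle (BP_dangban) and slides it along the Y axis toward where the mouse points.
; Pressing the left button triggers a move and runs a 0.01-second looping timer that repeats it until release pauses it.
; Each move line-traces from the deprojected cursor, ignoring the paddle and drawing debug lines.
; On a hit, a Timeline restarts to lerp the paddle's Y to the hit point at fixed height.
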(event Custom|点击事件
  (|计算起点和终点，并移动))

(event Custom|CustomEvent
  (CallFunction|点击事件))

(event EventBeginPlay
  (Utilities|FlowControl|Sequence
    (:then_0
      (Variables|/Script/Engine.PlayerController|SetbShowMouseCursor (Game|GetPlayerController 0) true)
      (Actor|GetAllActorswithTag "ignoreProps"))
    (:then_1
      (bind _returnvalue (Game|SpawnActorfromClass "/Game/BP/gamemode/BP_dangban.BP_dangban_C" (Math|Transform|MakeTransform "0, 0, 0" "0, 0, 0" "1.000000,1.000000,1.000000") "Undefined" "MultiplyWithRoot" 0 0))
      (bind _output_get (Variables|Default|SetDangBan _returnvalue))
      (Utilities|Array|Add (Variables|Default|GetActors%20to%20Ignore) _output_get))))

(event Input|MouseEvents|LeftMouseButton
  (params (Key :type Key%20Structure :default "None"))
  (:Pressed
    (Variables|Default|SetClicked true)
    (CallFunction|点击事件)
    (if (Class|KismetSystemLibrary|IsTimerPausedHandle (Variables|Default|GetClickTimerHandle))
      (Utilities|Time|UnpauseTimerbyHandle (Variables|Default|GetClickTimerHandle))
      (else
        (bind _returnvalue (Utilities|Time|SetTimerbyEvent (delegate Custom|CustomEvent) 0.01 true))
        (Variables|Default|SetClickTimerHandle _returnvalue))))
  (:Released
    (Variables|Default|SetClicked false)
    (Utilities|Time|PauseTimerbyHandle (Variables|Default|GetClickTimerHandle))))

(fn ConstructionScript)